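; Moon actor for a day/night cycle, with transition events that play the DayToNight timeline forward for night and in reverse for day.
; Logic to apply the timeline's tracks to moon opacity, glow density, directional light intensity and Fog parameter collection opacity exists, but is marked as never run.
; The construction script turns the actor to face an Origin point and applies a uniform Scale.
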(event `NightTransition`
  (bind (_direction _moon _glow _post_process _directionlight) (`Timeline|DayToNight` :!label _label)))

(event `Day Transition`
  (goto _label :!via `Reverse`))

(fn `UserConstructionScript`
  (bind _scale (`self.Scale`))
  (`self.K2_SetActorRotation` (`KismetMathLibrary.Conv_VectorToRotator` (`KismetMathLibrary.Normal` (- (`self.Origin`) (`self.K2_GetActorLocation`)))))
  (`self.SetActorScale3D` (`KismetMathLibrary.MakeVector` _scale _scale _scale)))