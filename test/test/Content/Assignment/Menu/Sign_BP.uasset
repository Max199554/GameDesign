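; Sign actor that shows editable text in the world and toggles an on-screen tips widget when interacted with.
; The construction script writes TextToRender into its text render component.
; The interact event removes the tips widget if one exists, otherwise creates one for the first player, adds it to the viewport and passes MyText as its dialogue text.
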(event `Interact_1`
  (bind _tipswidget (`self.TipsWidget`))
  (`/Engine/EditorBlueprintResources/StandardMacros.IsValid` (`self.TipsWidget`)
    (:`Is Valid`
      (`Widget.RemoveFromParent` _tipswidget)
      (set `self.TipsWidget` null))
    (:`Is Not Valid`
      (`Widget.RemoveFromParent` _tipswidget)
      (bind _returnvalue (`|CreateWidget` "/Game/Assignment/Menu/Tipswidget.Tipswidget_C" (`GameplayStatics.GetPlayerController` 0)))
      (bind _output_get (set `self.TipsWidget` _returnvalue))
      (`UserWidget.AddToViewport` _output_get 0)
      (set `/Game/Assignment/Menu/Tipswidget.DialoglueText` (`self.MyText`) (`self.TipsWidget`)))))

(fn `UserConstructionScript`
  (`TextRenderComponent.K2_SetText` (`self.TextRender`) (`self.TextToRender`)))