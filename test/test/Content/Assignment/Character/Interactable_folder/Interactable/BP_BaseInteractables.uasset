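; Base Blueprint for interactable objects that BP_Character can detect by proximity.
; Overlap begin and end on InteractableArea register and unregister the object with the overlapping BP_Character.
; SetHightLight toggles custom depth rendering on InteractableMesh for highlighting.
; GetContent is an empty stub that returns nothing here.
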(event `self.InteractableArea.OnComponentBeginOverlap`
  (params (OverlappedComponent :type "PrimitiveComponent Object Reference") (OtherActor :type "Actor Object Reference") (OtherComp :type "PrimitiveComponent Object Reference") (OtherBodyIndex :type Integer) (bFromSweep :type Boolean) (SweepResult :type "HitResult Structure (by ref)"))
  (bind _asbp_character (cast `/Game/Assignment/Character/BP_Character` OtherActor))
  (message `/Game/Assignment/Character/Interactable_folder/Interactable/BPI_Interactables.RegisterInteractable` _asbp_character self))

(event `self.InteractableArea.OnComponentEndOverlap`
  (params (OverlappedComponent :type "PrimitiveComponent Object Reference") (OtherActor :type "Actor Object Reference") (OtherComp :type "PrimitiveComponent Object Reference") (OtherBodyIndex :type Integer))
  (bind _asbp_character (cast `/Game/Assignment/Character/BP_Character` OtherActor))
  (message `/Game/Assignment/Character/Interactable_folder/Interactable/BPI_Interactables.UnRegisterInteractable` _asbp_character self))

(fn `Get Content`
  (returns (Content :type "/Game/UI_Kit/Blueprints/Actionbar/ActionbarSlotContent Structure") (Content :type "/Game/UI_Kit/Blueprints/Actionbar/ActionbarSlotContent Structure"))
  (return))

(fn `SetHightLight`
  (params (`HeightLight?` :type Boolean))
  (`PrimitiveComponent.SetRenderCustomDepth` (`self.Interactable_Mesh`) `HeightLight?`))

(fn `UserConstructionScript`)