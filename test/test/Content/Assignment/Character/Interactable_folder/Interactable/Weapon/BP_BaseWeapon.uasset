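; BP_BaseWeapon is the base melee-style weapon for the player character, with range, damage and hit effects read from WeaponInfo.
; Attack sphere-traces forward from the player, then damages enemies hit and spawns VFX and sound.
; For Character_Peoples1 targets, low health triggers a death camera shake; otherwise it sets Front, plays a combat shake and slows global time.
; Tick ramps time dilation back up, creating a brief hit-stop.
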(event `self.ReceiveTick`
  (params (DeltaSeconds :type "Float (single-precision)"))
  (if (< (`GameplayStatics.GetGlobalTimeDilation`) 1.0)
    (`GameplayStatics.SetGlobalTimeDilation` (+ (`GameplayStatics.GetGlobalTimeDilation`) 0.05))))

(event `self.ReceiveBeginPlay`
  (bind _asbp_character (cast `/Game/Assignment/Character/BP_Character` (`GameplayStatics.GetPlayerCharacter` 0)))
  (set `self.CharacterReference` _asbp_character))

(event `Attack`
  (bind (_weaponinfo_attacktype _weaponinfo_damage _weaponinfo_range) (break `/Game/Assignment/Character/Interactable_folder/Interactable/Weapon/FWeaponInfor` (`self.WeaponInfo`)))
  (bind _characterreference (`self.CharacterReference`))
  (bind ((`Damage_5_209A376F4CCA1A2BA5B04C97804ABFDB` _damage) (`HitVFX_32_F42C78224AB43A7B7C87EBB93B3D320C` _hitvfx) (`HitSFX_33_2E9A5C35488A1B5C625D3997CDFFFFA8` _hitsfx)) (break `/Game/Assignment/Character/Interactable_folder/Interactable/Weapon/FWeaponInfor` (`self.WeaponInfo`)))
  (bind _returnvalue (`self.K2_GetActorLocation` _characterreference))
  (bind (_outhits _returnvalue_2) (`KismetSystemLibrary.SphereTraceMulti` _returnvalue (+ _returnvalue (* (`self.GetActorForwardVector` _characterreference) _weaponinfo_range)) 25.0 "TraceTypeQuery2" false (`|MakeArray` _characterreference :!type "Actor Object Reference") "ForDuration"))
  (if _returnvalue_2
    (for _array_element _outhits
      (bind (_bblockinghit _binitialoverlap _time _distance _location _impactpoint _normal _impactnormal _physmat _hitactor) (`GameplayStatics.BreakHitResult` _array_element))
      (bind _asenemy_character (cast `EnemyCharacter` _hitactor))
      (`GameplayStatics.SpawnEmitterAtLocation` _hitvfx _location)
      (`GameplayStatics.PlaySoundAtLocation` _hitsfx _location (struct) 1.0 1.0 0.0 null null null)
      (bind _returnvalue_3 (`GameplayStatics.ApplyDamage` _asenemy_character _damage null (`self.CharacterReference`)))
      (`EnemyCharacter.TakeDamage` _asenemy_character _returnvalue_3)
      (bind _ascharacter_peoples_1 (cast `/Game/Assignment/Character_Peoples/Knight/Character_Peoples1` _asenemy_character))
      (if (<= (`EnemyCharacter.health` _ascharacter_peoples_1) 1.0)
        (`PlayerCameraManager.PlayCameraShake` :`self` (`GameplayStatics.GetPlayerCameraManager` 0) :`ShakeClass` "/Game/Assignment/DeathCamShake.DeathCamShake_C" :`Scale` 2.0)
        (else
          (set `/Game/Assignment/Character_Peoples/Knight/Character_Peoples1.Front` true _ascharacter_peoples_1)
          (`PlayerCameraManager.PlayCameraShake` :`self` (`GameplayStatics.GetPlayerCameraManager` 0) :`ShakeClass` "/Game/Assignment/CombatShake.CombatShake_C" :`Scale` 2.0)
          (`GameplayStatics.SetGlobalTimeDilation` 0.05))))))

(fn `UserConstructionScript`
  (`parent.UserConstructionScript`))