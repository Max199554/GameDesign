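; Base Blueprint for interactable items that can be picked up into the interacting actor's inventory.
; On Interaction, it checks the instigator for inventory space, passes its item info struct through PickUpMessage, then destroys itself.
; The construction script rebuilds that struct with the item's own class, keeping the other fields, so the picked-up data records which class it came from.
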(event `/Game/Assignment/Character/Interactable_folder/Interactable/BPI_Interactables.Interaction`
  (params (Insigator :type "/Game/Assignment/Character/BP_Character Object Reference"))
  (if (`/Game/Assignment/Character/BP_Character.HasSpaceInventory` Insigator)
    (message `/Game/Assignment/Character/Interactable_folder/Interactable/BPI_Interactables.PickUp` Insigator (`self.ItemInfor`))
    (`self.K2_DestroyActor`)))

(fn `UserConstructionScript`
  (bind (_iteminfor_itemtype _iteminfor_itemname _iteminfor_itemimage _iteminfor_itemclass _iteminfor_itemindex _iteminfor_itemslot _iteminfor_itemvalue) (break `/Game/Assignment/Character/Interactable_folder/Interactable/FItemInfor` (`self.ItemInfor`)))
  (`parent.UserConstructionScript`)
  (set `self.ItemInfor` (make `/Game/Assignment/Character/Interactable_folder/Interactable/FItemInfor` _iteminfor_itemtype _iteminfor_itemname _iteminfor_itemimage (`GameplayStatics.GetObjectClass` self) _iteminfor_itemindex _iteminfor_itemslot _iteminfor_itemvalue)))