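; AI controller for showcase enemies that runs the BT_Enemy behavior tree against the player pawn.
; On begin play it stores the player as Enemy and the controlled Example_Enemy's guard point in the BB_Enemy blackboard.
; Perception updates on the player set the perceived flag and save a nav-projected search location.
; Losing sight raises a search flag, which a timer clears after a fixed delay.
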(event `self.ReceiveBeginPlay`
  (`self.UseBlackboard` "/Game/UI_Kit/Showcase/Blueprints/AI/BB_Enemy.BB_Enemy")
  (`self.RunBehaviorTree` "/Game/UI_Kit/Showcase/Blueprints/AI/BT_Enemy.BT_Enemy")
  (`self.Set Enemy`)
  (`self.Set Guard Point`))

(event `self.AIPerception.OnPerceptionUpdated`
  (params (UpdatedActors :type "Array of Actor Object Reference (by ref)"))
  (for _array_element UpdatedActors
    (if (== _array_element (`self.Enemy`))
      (bind _info (`AIPerceptionComponent.GetActorsPerception` (`self.AIPerception`) (`self.Enemy`)))
      (`BlackboardComponent.SetValueAsVector` (`AIBlueprintHelperLibrary.GetBlackboard` null) (`self.BBKey_SearchLocation`) (`NavigationSystemV1.K2_ProjectPointToNavigation` (`self.K2_GetActorLocation` (`self.Enemy`)) null null (800.0 800.0 800.0)))
      (bind (_age _expirationage _strength _stimuluslocation _receiverlocation _tag _bsuccessfullysensed) (break `AIStimulus` (`|GetArrayItem` (`.LastSensedStimuli` (break `ActorPerceptionBlueprintInfo` _info)))))
      (`BlackboardComponent.SetValueAsBool` (`AIBlueprintHelperLibrary.GetBlackboard` null) (`self.BBKey_Perceived`) _bsuccessfullysensed)
      (if (not _bsuccessfullysensed)
        (`BlackboardComponent.SetValueAsBool` (`AIBlueprintHelperLibrary.GetBlackboard` null) (`self.BBKey_Search`) true)
        (`KismetSystemLibrary.K2_SetTimerDelegate` (delegate `Stop Searching`) 25.0)))))

(event `Stop Searching`
  (`BlackboardComponent.SetValueAsBool` (`AIBlueprintHelperLibrary.GetBlackboard` null) (`self.BBKey_Search`) false))

(fn `Set Enemy`
  (bind _output_get (set `self.Enemy` (`GameplayStatics.GetPlayerPawn` 0)))
  (`BlackboardComponent.SetValueAsObject` (`AIBlueprintHelperLibrary.GetBlackboard` null) (`self.BBKey_Enemy`) _output_get)
  (return))

(fn `Set Guard Point`
  (bind _asexample_enemy (cast `/Game/UI_Kit/Showcase/Blueprints/Example_Enemy` (`self.K2_GetPawn`))
    (:`then`
      (`BlackboardComponent.SetValueAsObject` (`AIBlueprintHelperLibrary.GetBlackboard` null) (`self.BBKey_GuardPoint`) (`/Game/UI_Kit/Showcase/Blueprints/Example_Enemy.Guard Point` _asexample_enemy))
      (return))
    (:`CastFailed`
      (return))))

(fn `UserConstructionScript`)